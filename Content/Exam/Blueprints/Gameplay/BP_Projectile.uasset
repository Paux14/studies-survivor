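; BP_Projectile is a reusable bullet actor that is switched on and off rather than destroyed.
; FireBullet sets the projectile movement velocity and enables query-only collision on the mesh.
; Every hit applies damage credited to the instigator and its controller, with the instigator as damage causer.
; Only hits on "Wall"-tagged actors zero the velocity, disable collision and broadcast OnBulletDestroyed with the bullet itself.
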(event OnComponentHit(ProjectileMesh)
  (params (HitComponent :type Primitive%20Component%20Object%20Reference) (OtherActor :type Actor%20Object%20Reference) (OtherComp :type Primitive%20Component%20Object%20Reference) (NormalImpulse :type Vector :default "0, 0, 0") (Hit :type Hit%20Result%20Structure%20%28by%20ref%29))
  (CallFunction|ApplyDamage OtherActor)
  (if (Actor|ActorHasTag OtherActor "Wall")
    (CallFunction|DesactivateBullet)
    (Default|CallOnBulletDestroyed self)))

(event Custom|FireBullet
  (params (Velocity :type Vector))
  (Variables|/Script/Engine.MovementComponent|SetVelocity (Variables|Default|GetProjectileMovement) Velocity)
  (Collision|SetCollisionEnabled (Variables|Default|GetProjectileMesh) "QueryOnly"))

(event Custom|DesactivateBullet
  (Variables|/Script/Engine.MovementComponent|SetVelocity (Variables|Default|GetProjectileMovement) "0, 0, 0")
  (Collision|SetCollisionEnabled (Variables|Default|GetProjectileMesh) "NoCollision"))

(fn ConstructionScript)

(fn ApplyDamage
  (params (DamagedActor :type Actor%20Object%20Reference))
  (bind _returnvalue (Game|GetInstigator))
  (Game|Damage|ApplyDamage DamagedActor (Variables|Gameplay|GetDamage) (Game|GetInstigatorController _returnvalue) _returnvalue "/Script/Engine.DamageType"))