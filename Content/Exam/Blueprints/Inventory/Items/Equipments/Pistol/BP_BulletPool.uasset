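; Bullet pool for the pistol that pre-spawns reusable BP_Projectile actors on its owner.
; On BeginPlay it spawns a configurable number of projectiles at the owner's location, disables their mesh collision, attaches them to the owner and stores them in BulletPool.
; Each projectile's OnBulletDestroyed dispatcher is bound to an event that moves it back to the owner and reattaches it, recycling it instead of spawning anew.
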(event Custom|OnBulletDestroyed_Event
  (params (BP_Projectile :type BP%20Projectile%20Object%20Reference))
  (bind _returnvalue (Components|GetOwner))
  (Transformation|SetActorLocation BP_Projectile (Transformation|GetActorLocation _returnvalue) false false)
  (Transformation|AttachActorToActor BP_Projectile _returnvalue "None" "KeepWorld" "KeepWorld" "KeepWorld" true))

(event EventBeginPlay
  (for _index (range 0 (Variables|Default|GetAmountOfBullet))
    (bind _returnvalue (Game|SpawnActorfromClass "/Game/Exam/Blueprints/Gameplay/BP_Projectile.BP_Projectile_C" (Math|Transform|MakeTransform (Transformation|GetActorLocation (Components|GetOwner)) "0, 0, 0" "1.000000,1.000000,1.000000") "Undefined" "MultiplyWithRoot" 0 0))
    (Collision|SetCollisionEnabled (Variables|/Game/Exam/Blueprints/Gameplay/BP_Projectile.BP_Projectile_C|GetProjectileMesh _returnvalue) "NoCollision")
    (Transformation|AttachActorToActor _returnvalue (Components|GetOwner) "None" "KeepWorld" "KeepWorld" "KeepWorld" true)
    (EventDispatchers|AssignOnBulletDestroyed _returnvalue (delegate Custom|OnBulletDestroyed_Event))
    (Utilities|Array|Add (Variables|Default|GetBulletPool) _returnvalue)))