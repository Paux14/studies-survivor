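; BP_Item is an inventory item pickup actor that disappears when the player touches it.
; Overlapping its SphereCollider with an actor tagged Player destroys it after a short delay; the item itself does not add anything to an inventory.
; IsEquipment checks whether an EquipmentComponent class is set, and GetItemType uses that result to return one of two item type enum values.
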(event OnComponentBeginOverlap(SphereCollider)
  (params (OverlappedComponent :type Primitive%20Component%20Object%20Reference) (OtherActor :type Actor%20Object%20Reference) (OtherComp :type Primitive%20Component%20Object%20Reference) (OtherBodyIndex :type Integer) (bFromSweep :type Boolean) (SweepResult :type Hit%20Result%20Structure%20%28by%20ref%29))
  (if (Actor|ActorHasTag OtherActor (Variables|Default|GetPlayer))
    (Utilities|FlowControl|Delay 0.1)
    (Actor|DestroyActor)))

(event EventBeginPlay)

(fn ConstructionScript)

(fn IsEquipment
  (return (Utilities|IsValidClass (Variables|Default|GetEquipmentComponent))))

(fn GetItemType
  (return (select (CallFunction|IsEquipment) "NewEnumerator1" "NewEnumerator0")))